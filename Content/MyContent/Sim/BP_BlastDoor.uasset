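; Blast door actor whose two panels cycle endlessly from BeginPlay, moving in opposite directions along local X at a slow speed, then reversing at a fast one.
; DoorMov runs both panels in parallel through latent MoveComponentTo chains, with only the left chain re-calling the event to loop.
; DeltaLeft and DeltaRight offset each panel's current relative location by DeltaDistance, keeping rotation unchanged.
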(event `self.ReceiveBeginPlay`
  (`self.DoorMov`))

(event `DoorMov`
  (bind _leftdoor (`self.LeftDoor`))
  (bind _rightdoor (`self.RightDoor`))
  (`|ExecutionSequence`
    (:`then_0`
      (bind (_newpos _newrot) (`self.DeltaLeft` (`self.LeftDoor`)))
      (`KismetSystemLibrary.MoveComponentTo` (`self.LeftDoor`) _newpos _newrot false false (`self.SpeedSlow`))
      (bind (_newpos_2 _newrot_2) (`self.DeltaRight` _leftdoor))
      (`KismetSystemLibrary.MoveComponentTo` _leftdoor _newpos_2 _newrot_2 false false (`self.SpeedFast`))
      (`self.DoorMov`))
    (:`then_1`
      (bind (_newpos_3 _newrot_3) (`self.DeltaRight` (`self.RightDoor`)))
      (`KismetSystemLibrary.MoveComponentTo` (`self.RightDoor`) _newpos_3 _newrot_3 false false (`self.SpeedSlow`))
      (bind (_newpos_4 _newrot_4) (`self.DeltaLeft` _rightdoor))
      (`KismetSystemLibrary.MoveComponentTo` _rightdoor _newpos_4 _newrot_4 false false (`self.SpeedFast`)))))

(fn `DeltaLeft`
  (params (MeshComponent :type "StaticMeshComponent Object Reference"))
  (returns (NewPos :type "Vector Structure") (NewRot :type "Rotator Structure"))
  (bind (_relativelocation_x _relativelocation_y _relativelocation_z) (`KismetMathLibrary.BreakVector` (`SceneComponent.RelativeLocation` MeshComponent)))
  (return (`KismetMathLibrary.MakeVector` (- _relativelocation_x (`self.DeltaDistance`)) _relativelocation_y _relativelocation_z) (`SceneComponent.RelativeRotation` MeshComponent)))

(fn `DeltaRight`
  (params (MeshComponent :type "StaticMeshComponent Object Reference"))
  (returns (NewPos :type "Vector Structure") (NewRot :type "Rotator Structure"))
  (bind (_relativelocation_x _relativelocation_y _relativelocation_z) (`KismetMathLibrary.BreakVector` (`SceneComponent.RelativeLocation` MeshComponent)))
  (return (`KismetMathLibrary.MakeVector` (+ _relativelocation_x (`self.DeltaDistance`)) _relativelocation_y _relativelocation_z) (`SceneComponent.RelativeRotation` MeshComponent)))

(fn `UserConstructionScript`)