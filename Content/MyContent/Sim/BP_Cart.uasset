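; BP_Cart is an actor that rides along the spline of its assigned PrTrack.
; On BeginPlay, if CartState is set, it plays the SimMoveCart timeline from CartStartOffset at a rate of one over DeltaVel.
; Each update maps the timeline alpha to a distance along the spline and sets the cart's world location and rotation to match.
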(event `self.ReceiveBeginPlay`
  (if (`self.CartState`)
    (`self.MoveCart`)))

(event `MoveCart`
  (bind _splinetrack (`/Game/MyContent/Sim/BP_Track.SplineTrack` (`self.PrTrack`)))
  (bind _returnvalue (`KismetMathLibrary.Lerp` 0.0 (`SplineComponent.GetSplineLength` _splinetrack) (`self.Alpha`)))
  (`TimelineComponent.SetPlayRate` (`self.SimMoveCart`) (/ 1.0 (`self.DeltaVel`)))
  (`TimelineComponent.SetNewTime` (`self.SimMoveCart`) (`self.CartStartOffset`))
  (bind (_direction _alpha) (`Timeline|SimMoveCart`)
    (:`Update`
      (set `self.Alpha` _alpha)
      (`self.K2_SetActorLocationAndRotation` (`SplineComponent.GetLocationAtDistanceAlongSpline` _splinetrack _returnvalue "World") (`SplineComponent.GetRotationAtDistanceAlongSpline` _splinetrack _returnvalue "World")))))

(fn `UserConstructionScript`)